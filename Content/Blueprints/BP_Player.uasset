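; BP_Player is a player Blueprint that handles basic look, movement and jump input.
; Turn and Lookup axes feed controller yaw and pitch.
; Horizontal and Vertical axes add movement along the right and forward vectors of the full control rotation, without isolating yaw.
; Pressing Jump calls Jump, while BeginPlay, overlap, Tick and the construction script do nothing.
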(event `self.ReceiveBeginPlay`)

(event `InputAxis|Turn`
  (params (AxisValue :type "Float (single-precision)"))
  (`self.AddControllerYawInput` AxisValue))

(event `InputAxis|Lookup`
  (params (AxisValue :type "Float (single-precision)"))
  (`self.AddControllerPitchInput` AxisValue))

(event `InputAxis|Horizontal`
  (params (AxisValue :type "Float (single-precision)"))
  (`self.AddMovementInput` (`KismetMathLibrary.GetRightVector` (`self.GetControlRotation`)) AxisValue))

(event `InputAxis|Vertical`
  (params (AxisValue :type "Float (single-precision)"))
  (`self.AddMovementInput` (`KismetMathLibrary.GetForwardVector` (`self.GetControlRotation`)) AxisValue))

(event `InputAction|Jump`
  (params (Key :type "Key Structure"))
  (:`Pressed`
    (`self.Jump`)))

(fn `UserConstructionScript`)